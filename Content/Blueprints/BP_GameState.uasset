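; BP_GameState is a game state that runs a timed match between two teams and decides the winner.
; On BeginPlay it waits for a delay read from BP_GameInstance, then resets both team scores.
; After a fixed ten-minute timer it compares the scores and prints a Team 1 win, Team 2 win or draw message.
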(event EventBeginPlay
  (Utilities|FlowControl|DelayUntilNextTick)
  (bind _asbp_game_instance (Utilities|Casting|CastToBP_GameInstance (Game|GetGameInstance)))
  (bind _output_get (Variables|Default|SetAs%20BP%20Game%20Instance _asbp_game_instance))
  (Utilities|FlowControl|Delay (Variables|/Game/Blueprints/BP_GameInstance.BP_GameInstance_C|GetDelayTime _output_get))
  (Variables|Default|SetTeam1Score 0)
  (Variables|Default|SetTeam2Score 0)
  (Development|PrintString "Reset Score")
  (Utilities|FlowControl|Delay 6e+02)
  (if (> (Variables|Default|GetTeam1Score) (Variables|Default|GetTeam2Score))
    (Development|PrintString "Team 1 Won")
    (elif (< (Variables|Default|GetTeam1Score) (Variables|Default|GetTeam2Score))
      (Development|PrintString "Team 2 Won")
      (else
        (Development|PrintString "Draw")))))

(fn ConstructionScript)