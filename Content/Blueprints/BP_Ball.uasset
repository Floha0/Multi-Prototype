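; BP_Ball is a ball actor that registers itself with nearby Team2 players as their annihilation target.
; On begin overlap, it casts the other actor to BP_ThirdPersonCharacter and, if its first tag is Team2, sets that character's AnnihilateObject to itself.
; On end overlap, the same check clears AnnihilateObject to None.
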(event Collision|EventActorEndOverlap
  (params (OtherActor :type Actor%20Object%20Reference))
  (bind _asbp_third_person_character (Utilities|Casting|CastToBP_ThirdPersonCharacter OtherActor))
  (if (== (Utilities|Array|Get(acopy) (Variables|/Script/Engine.Actor|GetTags _asbp_third_person_character)) "Team2")
    (Variables|/Game/ThirdPerson/Blueprints/BP_ThirdPersonCharacter.BP_ThirdPersonCharacter_C|SetAnnihilateObject _asbp_third_person_character 0)))

(event Collision|EventActorBeginOverlap
  (params (OtherActor :type Actor%20Object%20Reference))
  (bind _asbp_third_person_character (Utilities|Casting|CastToBP_ThirdPersonCharacter OtherActor))
  (if (== (Utilities|Array|Get(acopy) (Variables|/Script/Engine.Actor|GetTags _asbp_third_person_character)) "Team2")
    (Variables|/Game/ThirdPerson/Blueprints/BP_ThirdPersonCharacter.BP_ThirdPersonCharacter_C|SetAnnihilateObject _asbp_third_person_character self)))

(fn ConstructionScript)